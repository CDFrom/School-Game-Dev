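; BP_Button is a pressure plate that a BP_MyCube pushes down to open a tag-matched BP_MyDoor.
; Box overlaps drive two opposing MoveComponentTo nodes, each stopping the other before lowering or raising the platform.
; A completed press opens the door only if cube and button materials match; a completed release closes it.
; On Level1, both outcomes also show timed feedback messages through BP_FirstPersonGameMode.
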(event `self.Box.OnComponentBeginOverlap`
  (params (OverlappedComponent :type "PrimitiveComponent Object Reference") (OtherActor :type "Actor Object Reference") (OtherComp :type "PrimitiveComponent Object Reference") (OtherBodyIndex :type Integer) (bFromSweep :type Boolean) (SweepResult :type "HitResult Structure (by ref)"))
  (bind _sm_assetplatform (`self.SM_AssetPlatform`))
  (bind _sm_assetplatform_2 (`self.SM_AssetPlatform`))
  (bind _sm_assetplatform_3 (`self.SM_AssetPlatform`))
  (bind _output (`|GetArrayItem` (`Actor.Tags` (`ActorComponent.GetOwner` _sm_assetplatform_2))))
  ;[1 1 1] When the box is overlapped with a cube allow for the button to be pressed (moved) down over a set duration to a designate target height
  (if (== (`GameplayStatics.GetObjectClass` OtherActor) "/Game/Blueprints/BP_MyCube.BP_MyCube_C")
    (`|ExecutionSequence`
      (:`then_0`
        (goto _label_3 :!via `Stop`))
      (:`then_1`
        (`KismetSystemLibrary.MoveComponentTo` _sm_assetplatform_3 (`KismetMathLibrary.MakeVector` (.x (`SceneComponent.RelativeLocation` _sm_assetplatform_3)) (.y (`SceneComponent.RelativeLocation` _sm_assetplatform_3)) (`self.EndPos`)) (struct) false false (`self.Duration`) :!label _label)
        ;[1 1 1] After placing a cube on a button check if the colors (materials) match
        (bind _asbp_my_cube (cast `/Game/Blueprints/BP_MyCube` OtherActor))
        (if (== (`PrimitiveComponent.GetMaterial` (`/Game/Blueprints/BP_MyCube.Cube` _asbp_my_cube) 0) (`PrimitiveComponent.GetMaterial` _sm_assetplatform_2 0))
          ;[1 1 1] Get the tag of the button, find the door with that tag and open it
          (bind _outactors (`GameplayStatics.GetAllActorsOfClassWithTag` "/Game/Blueprints/BP_MyDoor.BP_MyDoor_C" _output))
          (`/Game/Blueprints/BP_MyDoor.OpenDoor` (`|GetArrayItem` _outactors))
          ;[1 1 1] Check if we are on level 1
          (bind _returnvalue (`GameplayStatics.GetCurrentLevelName` true))
          (if (`KismetStringLibrary.EqualEqual_StrStr` _returnvalue "Level1")
            ;[1 1 1] Based on the players actions set a message to display
            (if (== _output "Green")
              (set `self.Message` "Well done! Time to move on to the next stage. \nHead through the green door and we will begin.")
              (else
                (set `self.Message` "Not bad. But I am still not impressed.")))
            ;[1 1 1] Display the message for a set amount of time and then clear the screen
            (bind _asbp_first_person_game_mode (cast `/Game/FirstPerson/Blueprints/BP_FirstPersonGameMode` (`GameplayStatics.GetGameMode`) :!label _label_2))
            (set `/Game/FirstPerson/Blueprints/BP_FirstPersonGameMode.DisplayMessage` (`self.Message`) _asbp_first_person_game_mode)
            (`KismetSystemLibrary.Delay` (`self.MessageDuration`))
            (set `/Game/FirstPerson/Blueprints/BP_FirstPersonGameMode.DisplayMessage` "" _asbp_first_person_game_mode)))))))

(event `self.Box.OnComponentEndOverlap`
  (params (OverlappedComponent :type "PrimitiveComponent Object Reference") (OtherActor :type "Actor Object Reference") (OtherComp :type "PrimitiveComponent Object Reference") (OtherBodyIndex :type Integer))
  (bind _sm_assetplatform (`self.SM_AssetPlatform`))
  ;[1 1 1] When the box is no longer overlapped with a cube allow for the button to be lifted (moved) up over a set duration to a designate target height
  (if (== (`GameplayStatics.GetObjectClass` OtherActor) "/Game/Blueprints/BP_MyCube.BP_MyCube_C")
    (`|ExecutionSequence`
      (:`then_0`
        (goto _label :!via `Stop`))
      (:`then_1`
        (`KismetSystemLibrary.MoveComponentTo` _sm_assetplatform (`KismetMathLibrary.MakeVector` (.x (`SceneComponent.RelativeLocation` _sm_assetplatform)) (.y (`SceneComponent.RelativeLocation` _sm_assetplatform)) (`self.StartPos`)) (struct) false false (`self.Duration`) :!label _label_3)
        ;[1 1 1] If a cube is removed from the button close the door
        (bind _outactors (`GameplayStatics.GetAllActorsOfClassWithTag` "/Game/Blueprints/BP_MyDoor.BP_MyDoor_C" (`|GetArrayItem` (`Actor.Tags` (`ActorComponent.GetOwner` _sm_assetplatform)))))
        (`/Game/Blueprints/BP_MyDoor.CloseDoor` (`|GetArrayItem` _outactors))
        ;[1 1 1] Check if we are on level 1
        (bind _returnvalue (`GameplayStatics.GetCurrentLevelName` true))
        (if (`KismetStringLibrary.EqualEqual_StrStr` _returnvalue "Level1")
          ;[1 1 1] When the cube is picked up check if it was the same material as the button
          (bind _asbp_my_cube (cast `/Game/Blueprints/BP_MyCube` OtherActor))
          (if (== (`PrimitiveComponent.GetMaterial` (`/Game/Blueprints/BP_MyCube.Cube` _asbp_my_cube) 0) (`PrimitiveComponent.GetMaterial` (`self.SM_AssetPlatform`) 0))
            ;[1 1 1] Based on the players actions set a message to display
            (set `self.Message` "Leave the cube on the button...")
            (goto _label_2)
            (else
              (set `self.Message` "Yes, that is the wrong color.. the chimps were smarter..")
              (goto _label_2))))))))

(fn `UserConstructionScript`)