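; Ghost enemy character for a Pac-Man-style game that chases the player, turns edible when scared, and costs the player lives on contact.
; AI perception feeds target and line-of-sight blackboard keys through AIC_Ghost, with a short timer before losing a target.
; Scared state runs on a timer and slows movement.
; Capsule overlap either sends an eaten ghost to the origin frozen, or removes a life and resets everyone, or ends the game.
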(event `self.ReceiveBeginPlay`
  ;[1 1 1] Get the controller for the AI and get the current movement speed of the actor
  (set `self.AIController` (cast `/Game/AI/AIC_Ghost` (`self.GetController`) :!pure true))
  (set `self.MovementSpeed` (`CharacterMovementComponent.MaxWalkSpeed` (`self.CharacterMovement`))))

(event `SetScared`
  (bind _charactermovement (`self.CharacterMovement`))
  ;[1 1 1] Set the ghosts to scared for a set amount of time based on the timer
  (`KismetSystemLibrary.K2_ClearAndInvalidateTimerHandle` (`self.PowerUpTimer`))
  (`/Game/AI/AIC_Ghost.UpdateIsScaredKey` (`self.AIController`) true)
  (bind _returnvalue (`KismetSystemLibrary.K2_SetTimerDelegate` (delegate `SetNotScared`) 10.0))
  (set `self.PowerUpTimer` _returnvalue)
  (set `CharacterMovementComponent.MaxWalkSpeed` (- (`CharacterMovementComponent.MaxWalkSpeed` _charactermovement) (`self.VulnerableDebuff`)) _charactermovement))

(event `SetNotScared`
  (bind _charactermovement (`self.CharacterMovement`))
  ;[1 1 1] Set the ghosts to scared for a set amount of time based on the timer
  (`/Game/AI/AIC_Ghost.UpdateIsScaredKey` (`self.AIController`) false)
  (set `CharacterMovementComponent.MaxWalkSpeed` (+ (`self.VulnerableDebuff`) (`CharacterMovementComponent.MaxWalkSpeed` _charactermovement)) _charactermovement))

(event `self.AIPerception.OnTargetPerceptionUpdated`
  (params (Actor :type "Actor Object Reference") (Stimulus :type "AIStimulus Structure"))
  ;[1 1 1] Whenever the AI loses sight of a player begin a timer for losing that target actor and eventually stopping chase. Whenever an AI gains sight of a player, remove the timer for having lost the player and ensure that the AI has set the perceived actor to the player
  (if (== "/Game/ThirdPerson/Blueprints/BP_ThirdPersonCharacter.BP_ThirdPersonCharacter_C" (`GameplayStatics.GetObjectClass` Actor))
    (if (`.bSuccessfullySensed` (break `AIStimulus` Stimulus))
      (set `self.PerceivedActor` Actor)
      (`KismetSystemLibrary.K2_ClearAndInvalidateTimerHandle` (`self.TargetLostTimer`))
      (`/Game/AI/AIC_Ghost.UpdateTargetActorKey` (`self.AIController`) (`self.PerceivedActor`))
      (`/Game/AI/AIC_Ghost.UpdateHasLineOfSightKey` (`self.AIController`) true)
      (else
        (bind _returnvalue (`KismetSystemLibrary.K2_SetTimerDelegate` (delegate `TargetLost`) 2.0))
        (set `self.TargetLostTimer` _returnvalue)))))

(event `TargetLost`
  ;[1 1 1] Whenever the AI loses sight of a player begin a timer for losing that target actor and eventually stopping chase. Whenever an AI gains sight of a player, remove the timer for having lost the player and ensure that the AI has set the perceived actor to the player
  (set `self.PerceivedActor` null)
  (`/Game/AI/AIC_Ghost.UpdateTargetActorKey` (`self.AIController`) null)
  (`/Game/AI/AIC_Ghost.UpdateHasLineOfSightKey` (`self.AIController`) false))

(event `self.CapsuleComponent.OnComponentBeginOverlap`
  (params (OverlappedComponent :type "PrimitiveComponent Object Reference") (OtherActor :type "Actor Object Reference") (OtherComp :type "PrimitiveComponent Object Reference") (OtherBodyIndex :type Integer) (bFromSweep :type Boolean) (SweepResult :type "HitResult Structure (by ref)"))
  (bind _charactermovement (`self.CharacterMovement`))
  (bind _asbp_third_person_game_mode (cast `/Game/ThirdPerson/Blueprints/BP_ThirdPersonGameMode` (`GameplayStatics.GetGameMode`) :!pure true))
  (bind _asbp_third_person_character (cast `/Game/ThirdPerson/Blueprints/BP_ThirdPersonCharacter` (`GameplayStatics.GetPlayerCharacter` 0) :!pure true))
  (bind _asbp_third_person_game_mode_2 (cast `/Game/ThirdPerson/Blueprints/BP_ThirdPersonGameMode` (`GameplayStatics.GetGameMode`) :!pure true))
  (bind _lives (`/Game/ThirdPerson/Blueprints/BP_ThirdPersonGameMode.Lives` _asbp_third_person_game_mode))
  ;[1 1 1] Did we collide with the player
  (if (== (`GameplayStatics.GetObjectClass` OtherActor) "/Game/ThirdPerson/Blueprints/BP_ThirdPersonCharacter.BP_ThirdPersonCharacter_C")
    ;[1 1 1] Are we vulnerable/edible?
    (if (`BlackboardComponent.GetValueAsBool` (`AIBlueprintHelperLibrary.GetBlackboard` null) (`self.IsScaredKey`))
      ;[1 1 1] Move the ghost to the spawn, get points for 'eating' them and stop them from moving for a set time
      (`self.K2_SetActorLocation` (0.0 0.0 0.0))
      (if (not (`self.Eaten`))
        (set `self.Eaten` true)
        (`/Game/ThirdPerson/Blueprints/BP_ThirdPersonGameMode.AteGhost` (cast `/Game/ThirdPerson/Blueprints/BP_ThirdPersonGameMode` (`GameplayStatics.GetGameMode`) :!pure true)))
      (set `CharacterMovementComponent.MaxWalkSpeed` 0.0 _charactermovement)
      (`KismetSystemLibrary.Delay` 10.0)
      (set `CharacterMovementComponent.MaxWalkSpeed` (`self.MovementSpeed`) _charactermovement)
      (set `self.Eaten` false)
      (else
        ;[1 1 1] Check if the player has already been hit
        (if (not (`/Game/ThirdPerson/Blueprints/BP_ThirdPersonCharacter.HasBeenHit` _asbp_third_person_character))
          (set `/Game/ThirdPerson/Blueprints/BP_ThirdPersonCharacter.HasBeenHit` true _asbp_third_person_character)
          ;[1 1 1] Is player on last life?
          (if (<= _lives 1)
            ;[1 1 1] End Game
            (`/Game/ThirdPerson/Blueprints/BP_ThirdPersonGameMode.GameOver` _asbp_third_person_game_mode)
            (else
              ;[1 1 1] Remove a life, place all actors back to starting positions
              (`/Engine/EditorBlueprintResources/StandardMacros.DecrementInt` _lives
                (:`  `
                  (`/Game/ThirdPerson/Blueprints/BP_ThirdPersonGameMode.Caught` (cast `/Game/ThirdPerson/Blueprints/BP_ThirdPersonGameMode` (`GameplayStatics.GetGameMode`) :!pure true))
                  (`KismetSystemLibrary.Delay` 0.05)
                  (`self.K2_SetActorTransform` (`GameplayStatics.GetPlayerCharacter` 0) (`/Game/ThirdPerson/Blueprints/BP_ThirdPersonGameMode.PlayerStart` _asbp_third_person_game_mode_2) false false)
                  (bind _outactors (`GameplayStatics.GetAllActorsOfClass` "BP_AI_C"))
                  (for (_array_element _array_index) _outactors
                    (`self.K2_SetActorTransform` _array_element (`|GetArrayItem` (`/Game/ThirdPerson/Blueprints/BP_ThirdPersonGameMode.AIStart` _asbp_third_person_game_mode_2) _array_index) false false)
                    (set `/Game/ThirdPerson/Blueprints/BP_ThirdPersonCharacter.HasBeenHit` false (cast `/Game/ThirdPerson/Blueprints/BP_ThirdPersonCharacter` (`GameplayStatics.GetPlayerCharacter` 0) :!pure true))
                    (`/Game/ThirdPerson/Blueprints/BP_ThirdPersonGameMode.BeginGame` (cast `/Game/ThirdPerson/Blueprints/BP_ThirdPersonGameMode` (`GameplayStatics.GetGameMode`) :!pure true))))))))))))

(fn `UserConstructionScript`)