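; Points is a collectible pickup that awards score when the player walks over it and drives level progression.
; On overlap with player character 0, it destroys itself, then increases Score and PointsCollected on BP_ThirdPersonGameMode.
; When the collected count equals the game mode's PointsSpawned, it calls NextLevel on the game mode.
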(event `self.ReceiveActorBeginOverlap`
  (params (OtherActor :type "Actor Object Reference"))
  (bind _asbp_third_person_game_mode (cast `/Game/ThirdPerson/Blueprints/BP_ThirdPersonGameMode` (`GameplayStatics.GetGameMode`) :!pure true))
  ;[1 1 1] Upon walking over the point, destroy the actor
  (if (== OtherActor (`GameplayStatics.GetPlayerCharacter` 0))
    (`self.K2_DestroyActor`)
    ;[1 1 1] Update the points collected and if all the points have been collected, move to the next level
    (set `/Game/ThirdPerson/Blueprints/BP_ThirdPersonGameMode.Score` (+ (`/Game/ThirdPerson/Blueprints/BP_ThirdPersonGameMode.Score` _asbp_third_person_game_mode) 10) _asbp_third_person_game_mode)
    (bind _result (`/Engine/EditorBlueprintResources/StandardMacros.IncrementInt` (`/Game/ThirdPerson/Blueprints/BP_ThirdPersonGameMode.PointsCollected` _asbp_third_person_game_mode))
      (:`  `
        (if (== _result (`/Game/ThirdPerson/Blueprints/BP_ThirdPersonGameMode.PointsSpawned` _asbp_third_person_game_mode))
          (`/Game/ThirdPerson/Blueprints/BP_ThirdPersonGameMode.NextLevel` _asbp_third_person_game_mode))))))

(fn `UserConstructionScript`)