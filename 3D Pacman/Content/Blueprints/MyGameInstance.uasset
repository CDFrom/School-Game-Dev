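; Game instance that holds the game's Score, Time, Level and Lives values.
; On Init, a sequence casts the current game mode to BP_ThirdPersonGameMode and copies each value into its own variable, with Time taken from BaseTime.
; The copy happens only at Init, and nothing here writes values back to the game mode.
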(event `self.ReceiveInit`
  (bind _asbp_third_person_game_mode (cast `/Game/ThirdPerson/Blueprints/BP_ThirdPersonGameMode` (`GameplayStatics.GetGameMode`) :!pure true))
  (`|ExecutionSequence`
    (:`then_0`
      (set `self.Score` (`/Game/ThirdPerson/Blueprints/BP_ThirdPersonGameMode.Score` _asbp_third_person_game_mode)))
    (:`then_1`
      (set `self.Time` (`/Game/ThirdPerson/Blueprints/BP_ThirdPersonGameMode.BaseTime` _asbp_third_person_game_mode)))
    (:`then_2`
      (set `self.Level` (`/Game/ThirdPerson/Blueprints/BP_ThirdPersonGameMode.Level` _asbp_third_person_game_mode)))
    (:`then_3`
      (set `self.Lives` (`/Game/ThirdPerson/Blueprints/BP_ThirdPersonGameMode.Lives` _asbp_third_person_game_mode)))))